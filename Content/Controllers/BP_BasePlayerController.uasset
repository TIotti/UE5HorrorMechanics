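; BP_BasePlayerController is the player controller that manages the HUD, a time-based score and detection of enemies in view.
; On possess it adds the input mapping, creates the main widget and starts a looping score timer, paused on unpossess.
; Its pawn sensing component, with vision angle matched to half the camera's default FOV, flags seen enemies' AI controllers as detected for slightly longer than the sensing interval.
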(event `self.ReceiveBeginPlay`
  ;[1 1 1] Set pawn sensing's detection to half of the field of view
  (`PawnSensingComponent.SetPeripheralVisionAngle` (`self.PlayerPawnSensing`) (* (`PlayerCameraManager.DefaultFOV` (`GameplayStatics.GetPlayerCameraManager` 0)) 0.5)))

(event `OnScoreUpdated`
  ;[1 1 1] Update UI and what else should happen when score is updated
  (`/Engine/EditorBlueprintResources/StandardMacros.IsValid` (`self.PlayerWidget`)
    (:`Is Valid`
      (`/Game/Widgets/MainPlayerWidget.UpdateScore` (`self.PlayerWidget`) (`self.Score`)))))

(event `TriggerScoreEvent`
  ;[1 1 1] Score event as a background pausable process
  (bind _returnvalue (`KismetSystemLibrary.K2_SetTimer` null "IncrementScore" (`self.ScoreTime`) true))
  (set `self.ScoreUpdateTimeHandler` _returnvalue))

(event `SetupUI`
  ;[1 1 1] Client command to load UI and add on screen
  (bind _returnvalue (`|CreateWidget` "/Game/Widgets/MainPlayerWidget.MainPlayerWidget_C"))
  (bind _output_get (set `self.PlayerWidget` _returnvalue))
  (`UserWidget.AddToViewport` _output_get 0))

(event `self.ReceivePossess`
  (params (PossessedPawn :type "Pawn Object Reference"))
  ;[1 1 1] Posses
  (`EnhancedInputSubsystemInterface.AddMappingContext` (subsystem `EnhancedInputLocalPlayerSubsystem`) "/Game/Controllers/Input/IM_DefaultMapping.IM_DefaultMapping" 0 (make `ModifyContextOptions` true))
  (`self.SetupUI`)
  (`self.TriggerScoreEvent`))

(event `self.ReceiveUnPossess`
  (params (UnpossessedPawn :type "Pawn Object Reference"))
  ;[1 1 1] What should happen when player is died
  (`KismetSystemLibrary.K2_PauseTimerHandle` (`self.ScoreUpdateTimeHandler`)))

(event `self.PlayerPawnSensing.OnSeePawn`
  (params (Pawn :type "Pawn Object Reference"))
  ;[1 1 1] Detect Enemies on Sight
  (bind _asbp_enemy_controller (cast `/Game/Controllers/BP_EnemyController` (`AIBlueprintHelperLibrary.GetAIController` Pawn)))
  (`/Game/Controllers/BP_EnemyController.SetDetected` _asbp_enemy_controller (+ (`PawnSensingComponent.SensingInterval` (`self.PlayerPawnSensing`)) 0.5)))

(fn `IncrementScore`
  (`/Engine/EditorBlueprintResources/StandardMacros.IncrementInt` (`self.Score`)
    (:`  `
      (`self.OnScoreUpdated`))))

(fn `UserConstructionScript`)